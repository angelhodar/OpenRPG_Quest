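; Quest manager component that runs the player's RPG quests, from acquisition through completion, failure or cancellation.
; Quests spawn as actors from DT_Quests rows and move between per-state lists, updating the quest menu and tracked-quest widget.
; NPC talks and target interactions advance matching goals, while level-ups grant quests directly or through world NPCs.
; Quest progress saves to a QuestSave slot, and initialization respawns quests from it.
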(event Custom|OnTalkToNPC
  (params (NPC%20Class :type Actor%20Class%20Reference) (SpecificID :type Integer))
  (CallFunction|HandleTalktoNPC NPC%20Class SpecificID))

(event Custom|UpdateTrackedQuest
  (params (Quest :type BP%20Base%20Quest%20Object%20Reference))
  (bind _output_get (Variables|Default|SetCurrentTrackedQuest Quest))
  (Default|AssignNewQuest (Variables|Default|GetTrackedQuestWidget) _output_get)
  (Utilities|IsValid (Variables|Default|GetCurrentTrackedQuest)
    (:Is%20Valid
      (Default|CallOnQuestTracked (Default|GetQuestData (Variables|Default|GetCurrentTrackedQuest))))))

(event Custom|OnTargetInteraction
  (params (TargetClass :type Actor%20Class%20Reference))
  (CallFunction|HandleTargetInteracion TargetClass))

(event Custom|OnPlayerLvlUp
  (params (NewLvl :type Integer))
  (CallFunction|CheckNewQuestsonLvlUp NewLvl))

(event Custom|OnInteractWithNPC
  (bind _nearbynpcs (Variables|Default|GetNearbyNPCs))
  (bind _output (Utilities|Array|Get(acopy) _nearbynpcs))
  (Utilities|IsValid _output
    (:Is%20Valid
      (Default|OnInteract _output (Variables|Default|GetPlayer)))))

(event Custom|UpdateDisplayedQuest
  (params (Quest :type BP%20Base%20Quest%20Object%20Reference))
  (bind _output_get (Variables|Default|SetCurrentDisplayedQuest Quest))
  (Default|UpdateDisplayedQuest (Variables|Default|GetQuestMenu) _output_get))

(fn Initialize
  (params (Player :type Character%20Object%20Reference) (TrackQuest :type WB%20Tracked%20Quest%20Object%20Reference) (QuestMenu :type WB%20Quest%20Menu%20Object%20Reference))
  (Variables|Default|SetPlayer Player)
  (Variables|Default|SetTrackedQuestWidget TrackQuest)
  (bind _output_get (Variables|Default|SetQuestMenu QuestMenu))
  (Default|Initialize _output_get self)
  (bind _outactors (Actor|GetAllActorsOfClass "/Game/OpenRPG_QuestSystem/Blueprints/TestingClasses/BP_BaseNPC.BP_BaseNPC_C"))
  (Variables|Default|SetWorldNPCs _outactors)
  (CallFunction|LoadQuests)
  (return))

(fn AddNewQuest
  (params (QuestID :type Integer))
  (bind _output_get (LocalVariables|SetLocalQuestID QuestID))
  (bind _output_get_2 (LocalVariables|SetLocalQuestData (CallFunction|GetQuestDatafromID _output_get)))
  (bind _output_get_3 (LocalVariables|SetLocalQuestClass (Utilities|Struct|Breaks_QuestData _output_get_2)))
  (if (and (not (Utilities|Array|ContainsItem (Variables|Default|GetProcessedQuests) _output_get_3)) (Utilities|IsValidClass (LocalVariables|GetLocalQuestClass)))
    (Utilities|Array|Add (Variables|Default|GetProcessedQuests) (LocalVariables|GetLocalQuestClass))
    (bind _returnvalue (Game|SpawnActorfromClass (LocalVariables|GetLocalQuestClass) (Math|Transform|MakeTransform "0, 0, 0" "0, 0, 0" "1,1,1") "AlwaysSpawn" 0 (LocalVariables|GetLocalQuestID) (Variables|Default|GetPlayer) (LocalVariables|GetLocalQuestData) self 0))
    (bind _output_get_4 (LocalVariables|SetLocalNewQuest _returnvalue))
    (Default|Initialize _output_get_4 false)
    (Utilities|Array|Add (Variables|Default|GetActiveQuests) (LocalVariables|GetLocalNewQuest))
    (CallFunction|RemoveCanceledQuest (LocalVariables|GetLocalQuestClass))
    (Default|GenerateQuestEntries (Variables|Default|GetQuestMenu))
    (Default|CallOnQuestAdded (LocalVariables|GetLocalQuestData))
    (return)
    (else
      (Development|PrintString "Quest already added or not valid")
      (return))))

(fn IsQuestTracked?
  (params (Quest :type BP%20Base%20Quest%20Object%20Reference))
  (return (== Quest (Variables|Default|GetCurrentTrackedQuest))))

(fn IsQuestDisplayed?
  (params (Quest :type BP%20Base%20Quest%20Object%20Reference))
  (return (== Quest (Variables|Default|GetCurrentDisplayedQuest))))

(fn EndQuest
  (params (Quest :type BP%20Base%20Quest%20Object%20Reference) (FinalState :type e_QuestState%20Enum :default "NewEnumerator0"))
  (LocalVariables|SetLocalQuest Quest)
  (LocalVariables|SetLocalState FinalState)
  (Utilities|Array|RemoveItem (Variables|Default|GetActiveQuests) (LocalVariables|GetLocalQuest))
  (Default|SetNewState (LocalVariables|GetLocalQuest) (LocalVariables|GetLocalState))
  (Utilities|Array|Add (Utilities|Select :Index (LocalVariables|GetLocalState) :NewEnumerator0 (Variables|Default|GetActiveQuests) :NewEnumerator1 (Variables|Default|GetCompletedQuests) :NewEnumerator2 (Variables|Default|GetFailedQuests) :NewEnumerator3 (Variables|Default|GetCanceledQuests)) (LocalVariables|GetLocalQuest))
  (Default|GenerateQuestEntries (Variables|Default|GetQuestMenu))
  (if (CallFunction|IsQuestTracked? (LocalVariables|GetLocalQuest))
    (CallFunction|UpdateTrackedQuest))
  (if (CallFunction|IsQuestDisplayed? (LocalVariables|GetLocalQuest))
    (CallFunction|UpdateDisplayedQuest))
  (switch Utilities|FlowControl|Switch|Switchone_QuestState (LocalVariables|GetLocalState)
    (:NewEnumerator0
      (return))
    (:NewEnumerator1
      (Default|OnQuestCompleted (LocalVariables|GetLocalQuest))
      (Default|CallOnQuestCompleted (Default|GetQuestData (LocalVariables|GetLocalQuest)))
      (Default|CallOnRewardReceived (Utilities|Struct|Breaks_QuestData (Default|GetQuestData (LocalVariables|GetLocalQuest))))
      (return))
    (:NewEnumerator2
      (Default|OnQuestFailed (LocalVariables|GetLocalQuest))
      (Default|CallOnQuestFailed (Default|GetQuestData (LocalVariables|GetLocalQuest)))
      (return))
    (:NewEnumerator3
      (Utilities|Array|RemoveItem (Variables|Default|GetProcessedQuests) (Utilities|GetClass (LocalVariables|GetLocalQuest)))
      (Default|OnQuestCanceled (LocalVariables|GetLocalQuest))
      (Default|CallOnQuestCanceled (Default|GetQuestData (LocalVariables|GetLocalQuest)))
      (return))))

(fn GetQuestsbyFilter
  (params (Filter :type e_MenuFilter%20Enum :default "NewEnumerator0"))
  (bind _output_get (LocalVariables|SetLocalFilter Filter))
  (switch Utilities|FlowControl|Switch|Switchone_MenuFilter _output_get
    (:NewEnumerator0
      (Utilities|Array|AppendArray (LocalVariables|GetLocalFilteredQuests) (Variables|Default|GetActiveQuests))
      (Utilities|Array|AppendArray (LocalVariables|GetLocalFilteredQuests) (Variables|Default|GetCompletedQuests))
      (Utilities|Array|AppendArray (LocalVariables|GetLocalFilteredQuests) (Variables|Default|GetFailedQuests))
      (Utilities|Array|AppendArray (LocalVariables|GetLocalFilteredQuests) (Variables|Default|GetCanceledQuests))
      (return (LocalVariables|GetLocalFilteredQuests)))
    (:NewEnumerator1
      (LocalVariables|SetLocalCategory "NewEnumerator0"))
    (:NewEnumerator2
      (LocalVariables|SetLocalCategory "NewEnumerator1"))
    (:NewEnumerator3
      (LocalVariables|SetLocalCategory "NewEnumerator2"))
    (:NewEnumerator6
      (return (Variables|Default|GetActiveQuests)))
    (:NewEnumerator4
      (return (Variables|Default|GetCompletedQuests)))
    (:NewEnumerator5
      (return (Variables|Default|GetFailedQuests)))
    (:NewEnumerator7
      (return (Variables|Default|GetCanceledQuests))))
  (for _array_element (Variables|Default|GetActiveQuests)
    (if (Utilities|Enum|Equal(Enum) (Utilities|Struct|Breaks_QuestData (Variables|/Game/OpenRPG_QuestSystem/Blueprints/Quests/BP_BaseQuest.BP_BaseQuest_C|GetQuestData _array_element)) (LocalVariables|GetLocalCategory))
      (Utilities|Array|Add (LocalVariables|GetLocalFilteredQuests) _array_element)))
  (return (LocalVariables|GetLocalFilteredQuests)))

(fn ToggleQuestMenuVisibility
  (bind _questmenu (Variables|Default|GetQuestMenu))
  (if (Widget|IsVisible (Variables|Default|GetQuestMenu))
    (Widget|SetVisibility _questmenu "Hidden")
    (else
      (Widget|SetVisibility _questmenu "Visible")))
  (return))

(fn SearchNPC
  (params (Class :type Actor%20Class%20Reference) (SpecificID :type Integer))
  (LocalVariables|SetLocalClass Class)
  (LocalVariables|SetLocalID SpecificID)
  (bind _array_element (Utilities|Array|ForEachLoopwithBreak (Variables|Default|GetWorldNPCs) :!label _label)
    (:LoopBody
      (if (and (== (Utilities|GetClass _array_element) (LocalVariables|GetLocalClass)) (== (Variables|/Game/OpenRPG_QuestSystem/Blueprints/TestingClasses/BP_BaseNPC.BP_BaseNPC_C|GetID _array_element) (LocalVariables|GetLocalID)))
        (LocalVariables|SetLocalFoundNPC _array_element)
        (goto _label Break)))
    (:Completed
      (return (LocalVariables|GetLocalFoundNPC)))))

(fn HandleTalktoNPC
  (params (NPC%20Class :type Actor%20Class%20Reference) (SpecificID :type Integer))
  (LocalVariables|SetLocalClass NPC%20Class)
  (LocalVariables|SetLocalID SpecificID)
  (bind _array_element (Utilities|Array|ForEachLoopwithBreak (Variables|Default|GetActiveQuests) :!label _label)
    (:LoopBody
      (bind _output_get (LocalVariables|SetLocalQuest _array_element))
      (bind _array_element_2 (Utilities|Array|ForEachLoopwithBreak (Default|GetCurrentGoalIndices _output_get) :!label _label_2)
        (:LoopBody
          (if (Math|Boolean|ANDBoolean (Utilities|Enum|Equal(Enum) (.Type (Utilities|Struct|Breaks_GoalData (Default|GetGoalDataatIndex (LocalVariables|GetLocalQuest) _array_element_2))) "NewEnumerator2") (== (.TargetClass (Utilities|Struct|Breaks_GoalData (Default|GetGoalDataatIndex (LocalVariables|GetLocalQuest) _array_element_2))) (LocalVariables|GetLocalClass)) (== (.SpecificTargetID (Utilities|Struct|Breaks_GoalData (Default|GetGoalDataatIndex (LocalVariables|GetLocalQuest) _array_element_2))) (LocalVariables|GetLocalID)))
            (bind _success_ (Default|EndGoal (LocalVariables|GetLocalQuest) _array_element_2 false))
            (LocalVariables|SetLocalTalked _success_)
            (goto _label_2 Break)))
        (:Completed
          (if (LocalVariables|GetLocalTalked)
            (goto _label Break)))))
    (:Completed
      (return))))

(fn HandleTargetInteracion
  (params (TargetClass :type Actor%20Class%20Reference))
  (LocalVariables|SetLocalClass TargetClass)
  (for _array_element (Variables|Default|GetActiveQuests)
    (bind _output_get (LocalVariables|SetLocalQuest _array_element))
    (bind _array_element_2 (Utilities|Array|ForEachLoopwithBreak (Default|GetCurrentGoalIndices _output_get) :!label _label)
      (:LoopBody
        (bind _output_get_2 (LocalVariables|SetLocalGoal _array_element_2))
        (bind _output_get_3 (LocalVariables|SetLocalGoalData (Default|GetGoalDataatIndex (LocalVariables|GetLocalQuest) _output_get_2)))
        (if (and (Utilities|Enum|Equal(Enum) (.Type (Utilities|Struct|Breaks_GoalData _output_get_3)) "NewEnumerator1") (== (.TargetClass (Utilities|Struct|Breaks_GoalData _output_get_3)) (LocalVariables|GetLocalClass)))
          (Default|AddTargetAmount (LocalVariables|GetLocalQuest) (LocalVariables|GetLocalGoal) 1)
          (if (== (Utilities|Struct|Breaks_GoalData (LocalVariables|GetLocalGoalData)) (Default|GetGoalTargetAmount (LocalVariables|GetLocalQuest) (LocalVariables|GetLocalGoal)))
            (Default|EndGoal (LocalVariables|GetLocalQuest) (LocalVariables|GetLocalGoal) false)
            (goto _label Break)
            (else
              (Default|UpdateWidgets (LocalVariables|GetLocalQuest))))))))
  (return))

(fn AddNearbyNPC
  (params (NPC :type BP%20Base%20NPC%20Object%20Reference))
  (bind _output_get (LocalVariables|SetLocalNPC NPC))
  (if (Utilities|Array|ContainsItem (Variables|Default|GetNearbyNPCs) _output_get)
    (return)
    (else
      (Utilities|Array|Add (Variables|Default|GetNearbyNPCs) (LocalVariables|GetLocalNPC))
      (return))))

(fn RemoveNearbyNPC
  (params (NPC :type BP%20Base%20NPC%20Object%20Reference))
  (bind _output_get (LocalVariables|SetLocalNPC NPC))
  (if (Utilities|Array|ContainsItem (Variables|Default|GetNearbyNPCs) _output_get)
    (Utilities|Array|RemoveItem (Variables|Default|GetNearbyNPCs) (LocalVariables|GetLocalNPC))
    (return)
    (else
      (return))))

(fn RemoveCanceledQuest
  (params (Class :type BP%20Base%20Quest%20Class%20Reference))
  (LocalVariables|SetLocalClass Class)
  (bind (_arrayindex _arrayelement) (Utilities|Array|ReverseforEachLoop (Variables|Default|GetCanceledQuests))
    (:LoopBody
      (if (== (Utilities|GetClass _arrayelement) (LocalVariables|GetLocalClass))
        (Utilities|Array|RemoveIndex (Variables|Default|GetCanceledQuests) _arrayindex)))
    (:Completed
      (return))))

(fn GetQuestDatafromID
  (params (QuestID :type Integer))
  (bind _returnvalue (Utilities|GetDataTableRow "/Game/OpenRPG_QuestSystem/Blueprints/Quests/DT_Quests.DT_Quests" (Utilities|String|StringToName (Utilities|String|ToString(Integer) QuestID)))
    (:then
      (return _returnvalue))
    (:RowNotFound
      (return ""))))

(fn CheckNewQuestsonLvlUp
  (params (NewLvl :type Integer))
  (LocalVariables|SetLocalNewLvl NewLvl)
  (bind _array_element (Utilities|Array|ForEachLoopwithBreak (Variables|Configuration|GetQuestsPerLvl) :!label _label)
    (:LoopBody
      (if (== (.Lvl (Utilities|Struct|Breaks_QuestsPerLvl _array_element)) (LocalVariables|GetLocalNewLvl))
        (for _array_element_2 (.Quests (Utilities|Struct|Breaks_QuestsPerLvl _array_element))
          (bind _output_get (LocalVariables|SetLocalInfo _array_element_2))
          (if (Utilities|IsValidClass (Utilities|Struct|Breaks_QuestGiveData _output_get))
            (bind _npc (CallFunction|SearchNPC (.NPC (Utilities|Struct|Breaks_QuestGiveData (LocalVariables|GetLocalInfo))) (.SpecificID (Utilities|Struct|Breaks_QuestGiveData (LocalVariables|GetLocalInfo)))))
            (Utilities|IsValid _npc
              (:Is%20Valid
                (Default|ReceiveQuest _npc (Utilities|Struct|Breaks_QuestGiveData (LocalVariables|GetLocalInfo)))))
            (else
              (CallFunction|AddNewQuest (Utilities|Struct|Breaks_QuestGiveData (LocalVariables|GetLocalInfo))))))
        (goto _label Break)))
    (:Completed
      (return))))

(fn SaveQuests
  (Utilities|IsValid (Variables|Default|GetSaveQuestsClass)
    (:Is%20Valid
      _)
    (:Is%20Not%20Valid
      (bind _returnvalue (SaveGame|CreateSaveGameObject "/Game/OpenRPG_QuestSystem/Blueprints/QuestSave.QuestSave_C"))
      (Variables|Default|SetSaveQuestsClass _returnvalue)))
  (for _array_element (CallFunction|GetQuestsbyFilter "NewEnumerator0")
    (Utilities|Array|Add (Variables|/Game/OpenRPG_QuestSystem/Blueprints/QuestSave.QuestSave_C|GetSavedQuests (Variables|Default|GetSaveQuestsClass)) (Utilities|Struct|Makes_SavedQuest (Variables|/Game/OpenRPG_QuestSystem/Blueprints/Quests/BP_BaseQuest.BP_BaseQuest_C|GetID _array_element) (Default|GetCurrentState _array_element) (Variables|/Game/OpenRPG_QuestSystem/Blueprints/Quests/BP_BaseQuest.BP_BaseQuest_C|GetCurrentDescription _array_element) (Default|GetCurrentGoalIndices _array_element) (Default|GetCompletedGoalIndices _array_element) (Default|GetFailedGoalIndices _array_element) (Variables|/Game/OpenRPG_QuestSystem/Blueprints/Quests/BP_BaseQuest.BP_BaseQuest_C|GetCurrentTargetAmounts _array_element) (Variables|/Game/OpenRPG_QuestSystem/Blueprints/Quests/BP_BaseQuest.BP_BaseQuest_C|GetElapsedTimes _array_element))))
  (SaveGame|SaveGametoSlot (Variables|Default|GetSaveQuestsClass) (Variables|Default|GetSavedQuestsSlotName))
  (Development|PrintString "Quests Saved Succesfully!" true true "(R=0.000000,G=0.660000,B=1.000000,A=1.000000)" 5.0)
  (return))

(fn LoadQuests
  (Utilities|IsValid (Variables|Default|GetSaveQuestsClass)
    (:Is%20Valid
      _)
    (:Is%20Not%20Valid
      (bind _returnvalue (SaveGame|LoadGamefromSlot (Variables|Default|GetSavedQuestsSlotName)))
      (bind _asquest_save (Utilities|Casting|CastToQuestSave _returnvalue)
        (:then
          (Variables|Default|SetSaveQuestsClass _asquest_save))
        (:CastFailed
          (return)))))
  (for _array_element (Variables|/Game/OpenRPG_QuestSystem/Blueprints/QuestSave.QuestSave_C|GetSavedQuests (Variables|Default|GetSaveQuestsClass))
    (bind _returnvalue_2 (Game|SpawnActorfromClass (Utilities|Struct|Breaks_QuestData (CallFunction|GetQuestDatafromID (Utilities|Struct|Breaks_SavedQuest _array_element))) (Math|Transform|MakeTransform "0, 0, 0" "0, 0, 0" "1,1,1") "AlwaysSpawn" 0 (Utilities|Struct|Breaks_SavedQuest _array_element) (Variables|Default|GetPlayer) (CallFunction|GetQuestDatafromID (Utilities|Struct|Breaks_SavedQuest _array_element)) self 0))
    (Default|Initialize _returnvalue_2 true _array_element)
    (Utilities|Array|Add (Utilities|Select :Index (Utilities|Struct|Breaks_SavedQuest _array_element) :NewEnumerator0 (Variables|Default|GetActiveQuests) :NewEnumerator1 (Variables|Default|GetCompletedQuests) :NewEnumerator2 (Variables|Default|GetFailedQuests) :NewEnumerator3 (Variables|Default|GetCanceledQuests)) _returnvalue_2))
  (Default|GenerateQuestEntries (Variables|Default|GetQuestMenu))
  (Development|PrintString "Quests Loaded Succesfully!" true true "(R=0.000000,G=0.660000,B=1.000000,A=1.000000)" 5.0)
  (return))