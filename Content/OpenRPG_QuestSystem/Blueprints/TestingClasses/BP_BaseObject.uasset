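; Base interactable world object for the OpenRPG quest system that counts as a quest target when a player interacts with it.
; A sphere sized by InteractRadius in construction shows or hides an interact prompt widget, initialized with the object's text and R key, for overlapping actors with a BPC_QuestManager.
; OnInteract reports the object's class to the player's quest manager, then destroys the object.
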(event OnComponentBeginOverlap(InteractColision)
  (params (OverlappedComponent :type Primitive%20Component%20Object%20Reference) (OtherActor :type Actor%20Object%20Reference) (OtherComp :type Primitive%20Component%20Object%20Reference) (OtherBodyIndex :type Integer) (bFromSweep :type Boolean) (SweepResult :type Hit%20Result%20Structure%20%28by%20ref%29))
  (Utilities|IsValid (Actor|GetComponentbyClass OtherActor "/Game/OpenRPG_QuestSystem/Blueprints/BPC_QuestManager.BPC_QuestManager_C")
    (:Is%20Valid
      (Rendering|SetVisibility (Variables|Default|GetInteractWidget) true false))))

(event OnComponentEndOverlap(InteractColision)
  (params (OverlappedComponent :type Primitive%20Component%20Object%20Reference) (OtherActor :type Actor%20Object%20Reference) (OtherComp :type Primitive%20Component%20Object%20Reference) (OtherBodyIndex :type Integer))
  (Utilities|IsValid (Actor|GetComponentbyClass OtherActor "/Game/OpenRPG_QuestSystem/Blueprints/BPC_QuestManager.BPC_QuestManager_C")
    (:Is%20Valid
      (Rendering|SetVisibility (Variables|Default|GetInteractWidget) false false))))

(event Custom|OnInteract
  (params (Player :type Character%20Object%20Reference))
  (bind _output_get (Variables|Default|SetPlayer Player))
  (Utilities|IsValid (Actor|GetComponentbyClass _output_get "/Game/OpenRPG_QuestSystem/Blueprints/BPC_QuestManager.BPC_QuestManager_C")
    (:Is%20Valid
      (Default|OnTargetInteraction (Actor|GetComponentbyClass _output_get "/Game/OpenRPG_QuestSystem/Blueprints/BPC_QuestManager.BPC_QuestManager_C") (Utilities|GetClass self))
      (Actor|DestroyActor))))

(event EventBeginPlay
  (bind _aswb_interact_text (Utilities|Casting|CastToWB_InteractText (UserInterface|GetUserWidgetObject (Variables|Default|GetInteractWidget))))
  (bind _output_get (Variables|Default|SetInteractWidgetText _aswb_interact_text))
  (Default|Initialize _output_get (Variables|Default|GetText) "R")
  (Rendering|SetVisibility (Variables|Default|GetInteractWidget) false false))

(fn ConstructionScript
  (Components|Sphere|SetSphereRadius (Variables|Default|GetInteractColision) (Variables|Default|GetInteractRadius) true))