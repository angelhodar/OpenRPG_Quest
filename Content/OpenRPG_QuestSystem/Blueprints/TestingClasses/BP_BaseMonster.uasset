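; Test monster for the quest system that wanders and counts toward kill quests when damaged by a player.
; It loops AI moves to random reachable points around its spawn, pausing after each successful move.
; A radius-configurable sphere shows an interact prompt widget to overlapping actors that have a BPC_QuestManager.
; Any damage event from such a player reports the monster's class to that manager and destroys it, with no health check.
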(event OnComponentBeginOverlap(InteractColision)
  (params (OverlappedComponent :type Primitive%20Component%20Object%20Reference) (OtherActor :type Actor%20Object%20Reference) (OtherComp :type Primitive%20Component%20Object%20Reference) (OtherBodyIndex :type Integer) (bFromSweep :type Boolean) (SweepResult :type Hit%20Result%20Structure%20%28by%20ref%29))
  (Utilities|IsValid (Actor|GetComponentbyClass OtherActor "/Game/OpenRPG_QuestSystem/Blueprints/BPC_QuestManager.BPC_QuestManager_C")
    (:Is%20Valid
      (Rendering|SetVisibility (Variables|Default|GetInteractWidgetText) true false))))

(event OnComponentEndOverlap(InteractColision)
  (params (OverlappedComponent :type Primitive%20Component%20Object%20Reference) (OtherActor :type Actor%20Object%20Reference) (OtherComp :type Primitive%20Component%20Object%20Reference) (OtherBodyIndex :type Integer))
  (Utilities|IsValid (Actor|GetComponentbyClass OtherActor "/Game/OpenRPG_QuestSystem/Blueprints/BPC_QuestManager.BPC_QuestManager_C")
    (:Is%20Valid
      (Rendering|SetVisibility (Variables|Default|GetInteractWidgetText) false false))))

(event Custom|OnReceiveDamage
  (params (Player :type Character%20Object%20Reference))
  (bind _output_get (Variables|Default|SetPlayer Player))
  (Utilities|IsValid (Actor|GetComponentbyClass _output_get "/Game/OpenRPG_QuestSystem/Blueprints/BPC_QuestManager.BPC_QuestManager_C")
    (:Is%20Valid
      (Default|OnEnemyKilled (Actor|GetComponentbyClass _output_get "/Game/OpenRPG_QuestSystem/Blueprints/BPC_QuestManager.BPC_QuestManager_C") (Utilities|GetClass self))
      (Actor|DestroyActor))))

(event Custom|StartPatrolling
  (AI|AIMoveTo self (.RandomLocation (AI|Navigation|GetRandomReachablePointinRadius (Variables|Default|GetStartingLocation) 5e+02)) 0 5.0 false
    (:OnSuccess
      (Utilities|FlowControl|Delay 5.0)
      (CallFunction|StartPatrolling))))

(event EventBeginPlay
  (bind _aswb_interact_text (Utilities|Casting|CastToWB_InteractText (UserInterface|GetUserWidgetObject (Variables|Default|GetInteractWidgetText))))
  (bind _output_get (Variables|Default|SetInteractWidget _aswb_interact_text))
  (Default|Initialize _output_get (Variables|Default|GetText) "K")
  (Rendering|SetVisibility (Variables|Default|GetInteractWidgetText) false false)
  (Variables|Default|SetStartingLocation (Transformation|GetActorLocation))
  (CallFunction|StartPatrolling))

(fn ConstructionScript
  (Components|Sphere|SetSphereRadius (Variables|Default|GetInteractColision) (Variables|Default|GetInteractRadius) true))