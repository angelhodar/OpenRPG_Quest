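; Quest manager component for its owning player that adds, tracks, finishes, saves and loads quests.
; Quests spawn as actors from DT_Quests rows, and their state persists through a QuestSave slot.
; NPC talk and target interactions advance active goals, while level-ups offer quests through named NPCs or add them directly.
; Changes reach the quest list and interface-based detail widgets, and interaction rotates through nearby NPCs.
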(event Custom|OnTalkToNPC
  (params (NPC :type Name))
  (Interaction|HandleTalktoNPC NPC))

(event Custom|OnTargetInteraction
  (params (TargetName :type Name))
  (Interaction|HandleTargetInteracion TargetName))

(event Custom|OnPlayerLvlUp
  (params (NewLvl :type Integer))
  (Helpers|CheckNewQuestsonLvlUp NewLvl))

(event Custom|Initialize
  (Variables|Default|SetPlayer (Components|GetOwner))
  (Save/Load|LoadQuests)
  (bind _outactors (Actor|GetAllActorswithInterface "/Game/OpenRPG_QuestSystem/Blueprints/Interfaces/BPI_NPC.BPI_NPC_C"))
  (Variables|NPCs|SetWorldNPCs _outactors)
  (UI|InitializeWidgets))

(event Custom|OnInteractWithNPC
  (bind _npc (Helpers|GetFirstNPC))
  (Utilities|IsValid _npc
    (:Is%20Valid
      (Class|BPINPC|Interact(Message) _npc (Variables|Default|GetPlayer)))))

(fn AddNewQuest
  (params (Quest :type Name) (NPC :type Name))
  (LocalVariables|SetLocalQuestName Quest)
  (LocalVariables|SetLocalNPC NPC)
  (bind _output_get (LocalVariables|SetLocalQuestData (Helpers|GetQuestDatafromID (LocalVariables|GetLocalQuestName))))
  (bind _output_get_2 (LocalVariables|SetLocalQuestClass (Utilities|Struct|Breaks_QuestData _output_get)))
  (if (and (not (Helpers|QuestAlreadyAdded? _output_get_2)) (Utilities|IsValidClass (LocalVariables|GetLocalQuestClass)))
    (bind _returnvalue (Game|SpawnActorfromClass (LocalVariables|GetLocalQuestClass) (Math|Transform|MakeTransform "0, 0, 0" "0, 0, 0" "1,1,1") "AlwaysSpawn" 0 (LocalVariables|GetLocalQuestName) (LocalVariables|GetLocalNPC) (LocalVariables|GetLocalQuestData) (Variables|Default|GetPlayer) self 0))
    (bind _output_get_3 (LocalVariables|SetLocalNewQuest _returnvalue))
    (Default|Initialize _output_get_3)
    (Utilities|Array|Add (Variables|Quests|GetQuests) (LocalVariables|GetLocalNewQuest))
    (UI|UpdateQuestsList)
    (Default|CallOnQuestAdded (LocalVariables|GetLocalNewQuest))
    (return)
    (else
      (Development|PrintString "Quest already added or not valid")
      (return))))

(fn IsQuestSelected?
  (params (Quest :type BP%20Base%20Quest%20Object%20Reference))
  (return (== Quest (Variables|Quests|GetCurrentSelectedQuest))))

(fn EndQuest
  (params (Quest :type BP%20Base%20Quest%20Object%20Reference) (FinalState :type e_QuestState%20Enum :default "NewEnumerator0"))
  (LocalVariables|SetLocalQuest Quest)
  (bind _output_get (LocalVariables|SetLocalState FinalState))
  (Variables|/Game/OpenRPG_QuestSystem/Blueprints/Quests/BP_BaseQuest.BP_BaseQuest_C|SetState (LocalVariables|GetLocalQuest) _output_get)
  (UI|UpdateFinishedQuest (LocalVariables|GetLocalQuest))
  (switch Utilities|FlowControl|Switch|Switchone_QuestState (LocalVariables|GetLocalState)
    (:NewEnumerator0
      (return))
    (:NewEnumerator1
      (Default|OnQuestCompleted (LocalVariables|GetLocalQuest)))
    (:NewEnumerator2
      (Default|OnQuestFailed (LocalVariables|GetLocalQuest)))
    (:NewEnumerator3
      (Default|OnQuestCanceled (LocalVariables|GetLocalQuest))))
  (Default|CallOnQuestFinished (LocalVariables|GetLocalQuest))
  (return))

(fn ToggleQuestMenuVisibility
  (bind _questjournal (Variables|UI|GetQuestJournal))
  (if (Widget|IsVisible (Variables|UI|GetQuestJournal))
    (Widget|SetVisibility _questjournal "Hidden")
    (else
      (Widget|SetVisibility _questjournal "Visible")))
  (return))

(fn SearchNPC
  (params (NPC :type Name))
  (LocalVariables|SetLocalNPC NPC)
  (bind _array_element (Utilities|Array|ForEachLoopwithBreak (Variables|NPCs|GetWorldNPCs) :!label _label)
    (:LoopBody
      (bind _name (Class|BPINPC|GetName(Message) _array_element))
      (if (Utilities|Name|Equal(Name) _name (LocalVariables|GetLocalNPC))
        (LocalVariables|SetLocalFoundNPC _array_element)
        (goto _label Break)))
    (:Completed
      (return (LocalVariables|GetLocalFoundNPC)))))

(fn HandleTalktoNPC
  (params (NPC :type Name))
  (LocalVariables|SetLocalNPC NPC)
  (bind _array_element (Utilities|Array|ForEachLoopwithBreak (Variables|Quests|GetQuests) :!label _label)
    (:LoopBody
      (bind _output_get (LocalVariables|SetLocalQuest _array_element))
      (if (Utilities|Enum|Equal(Enum) (Variables|/Game/OpenRPG_QuestSystem/Blueprints/Quests/BP_BaseQuest.BP_BaseQuest_C|GetState _output_get) "NewEnumerator0")
        (bind _array_element_2 (Utilities|Array|ForEachLoopwithBreak (Variables|/Game/OpenRPG_QuestSystem/Blueprints/Quests/BP_BaseQuest.BP_BaseQuest_C|GetCurrentGoalIndices (LocalVariables|GetLocalQuest)) :!label _label_2)
          (:LoopBody
            (if (and (Utilities|Enum|Equal(Enum) (.Type (Utilities|Struct|Breaks_GoalData (Default|GetGoalDataatIndex (LocalVariables|GetLocalQuest) _array_element_2))) "NewEnumerator2") (Utilities|Name|Equal(Name) (.Target (Utilities|Struct|Breaks_GoalData (Default|GetGoalDataatIndex (LocalVariables|GetLocalQuest) _array_element_2))) (LocalVariables|GetLocalNPC)))
              (bind _success_ (Default|EndGoal (LocalVariables|GetLocalQuest) _array_element_2 false))
              (LocalVariables|SetLocalTalked _success_)
              (goto _label_2 Break)))
          (:Completed
            (if (LocalVariables|GetLocalTalked)
              (goto _label Break))))))
    (:Completed
      (return))))

(fn HandleTargetInteracion
  (params (TargetName :type Name))
  (LocalVariables|SetLocalTarget TargetName)
  (for _array_element (Variables|Quests|GetQuests)
    (bind _output_get (LocalVariables|SetLocalQuest _array_element))
    (if (Utilities|Enum|Equal(Enum) (Variables|/Game/OpenRPG_QuestSystem/Blueprints/Quests/BP_BaseQuest.BP_BaseQuest_C|GetState _output_get) "NewEnumerator0")
      (bind _array_element_2 (Utilities|Array|ForEachLoopwithBreak (Variables|/Game/OpenRPG_QuestSystem/Blueprints/Quests/BP_BaseQuest.BP_BaseQuest_C|GetCurrentGoalIndices (LocalVariables|GetLocalQuest)) :!label _label)
        (:LoopBody
          (bind _output_get_2 (LocalVariables|SetLocalGoal _array_element_2))
          (bind _output_get_3 (LocalVariables|SetLocalGoalData (Default|GetGoalDataatIndex (LocalVariables|GetLocalQuest) _output_get_2)))
          (if (and (Utilities|Enum|Equal(Enum) (.Type (Utilities|Struct|Breaks_GoalData _output_get_3)) "NewEnumerator1") (Utilities|Name|Equal(Name) (.Target (Utilities|Struct|Breaks_GoalData _output_get_3)) (LocalVariables|GetLocalTarget)))
            (Default|AddGoalTargetAmount (LocalVariables|GetLocalQuest) (LocalVariables|GetLocalGoal) 1)
            (if (== (Utilities|Struct|Breaks_GoalData (LocalVariables|GetLocalGoalData)) (Default|GetGoalTargetAmount (LocalVariables|GetLocalQuest) (LocalVariables|GetLocalGoal)))
              (Default|EndGoal (LocalVariables|GetLocalQuest) (LocalVariables|GetLocalGoal) false)
              (goto _label Break)
              (else
                (UI|UpdateQuestGoalWidget (LocalVariables|GetLocalQuest) (LocalVariables|GetLocalGoal)))))))))
  (return))

(fn AddNearbyNPC
  (params (NPC :type Actor%20Object%20Reference))
  (bind _output_get (LocalVariables|SetLocalNPC NPC))
  (if (Utilities|Array|ContainsItem (Variables|NPCs|GetNearbyNPCs) _output_get)
    (return)
    (else
      (Utilities|Array|Add (Variables|NPCs|GetNearbyNPCs) (LocalVariables|GetLocalNPC))
      (return))))

(fn RemoveNearbyNPC
  (params (NPC :type Actor%20Object%20Reference))
  (bind _output_get (LocalVariables|SetLocalNPC NPC))
  (if (Utilities|Array|ContainsItem (Variables|NPCs|GetNearbyNPCs) _output_get)
    (Utilities|Array|RemoveItem (Variables|NPCs|GetNearbyNPCs) (LocalVariables|GetLocalNPC))
    (return)
    (else
      (return))))

(fn GetQuestDatafromID
  (params (Quest :type Name))
  (bind _returnvalue (Utilities|GetDataTableRow "/Game/OpenRPG_QuestSystem/Datatables/DT_Quests.DT_Quests" Quest)
    (:then
      (return _returnvalue))
    (:RowNotFound
      (return ""))))

(fn CheckNewQuestsonLvlUp
  (params (NewLvl :type Integer))
  (LocalVariables|SetLocalNewLvl NewLvl)
  (bind _array_element (Utilities|Array|ForEachLoopwithBreak (Variables|Settings|GetQuestsPerLvl) :!label _label)
    (:LoopBody
      (if (== (.Lvl (Utilities|Struct|Breaks_QuestsPerLvl _array_element)) (LocalVariables|GetLocalNewLvl))
        (for _array_element_2 (.Quests (Utilities|Struct|Breaks_QuestsPerLvl _array_element))
          (bind _output_get (LocalVariables|SetLocalQuestData _array_element_2))
          (if (Utilities|Name|NotEqual(Name) (Utilities|Struct|Breaks_QuestReceiving _output_get) "None")
            (bind _npc_reference (NPCs|SearchNPC (Utilities|Struct|Breaks_QuestReceiving (LocalVariables|GetLocalQuestData))))
            (Utilities|IsValid _npc_reference
              (:Is%20Valid
                (Class|BPINPC|ReceiveQuest(Message) _npc_reference (Utilities|Struct|Breaks_QuestReceiving (LocalVariables|GetLocalQuestData)))
                (Default|CallOnNewQuestAvailable)
                (return))
              (:Is%20Not%20Valid
                (Development|PrintString (Utilities|String|Append "The NPC " (Utilities|String|ToString(Name) (Utilities|Struct|Breaks_QuestReceiving (LocalVariables|GetLocalQuestData))) " is not valid"))))
            (else
              (Managment|AddNewQuest (Utilities|Struct|Breaks_QuestReceiving (LocalVariables|GetLocalQuestData)) "None"))))
        (goto _label Break)))
    (:Completed
      (return))))

(fn SaveQuests
  (Utilities|IsValid (Variables|Save/Load|GetSaveQuestsClass)
    (:Is%20Valid
      _)
    (:Is%20Not%20Valid
      (bind _returnvalue (SaveGame|CreateSaveGameObject "/Game/OpenRPG_QuestSystem/Blueprints/QuestSave.QuestSave_C"))
      (Variables|Save/Load|SetSaveQuestsClass _returnvalue)))
  (for _array_element (Variables|Quests|GetQuests)
    (bind _output_get (LocalVariables|SetLocalQuest _array_element))
    (Default|UpdateGoalsRemainingTime _output_get)
    (Utilities|Array|Add (Variables|/Game/OpenRPG_QuestSystem/Blueprints/QuestSave.QuestSave_C|GetSavedQuests (Variables|Save/Load|GetSaveQuestsClass)) (Utilities|Struct|Makes_SavedQuest (Variables|/Game/OpenRPG_QuestSystem/Blueprints/Quests/BP_BaseQuest.BP_BaseQuest_C|GetQuestName (LocalVariables|GetLocalQuest)) (Variables|/Game/OpenRPG_QuestSystem/Blueprints/Quests/BP_BaseQuest.BP_BaseQuest_C|GetState (LocalVariables|GetLocalQuest)) (Variables|/Game/OpenRPG_QuestSystem/Blueprints/Quests/BP_BaseQuest.BP_BaseQuest_C|GetCurrentDescription (LocalVariables|GetLocalQuest)) (Variables|/Game/OpenRPG_QuestSystem/Blueprints/Quests/BP_BaseQuest.BP_BaseQuest_C|GetCurrentGoalIndices (LocalVariables|GetLocalQuest)) (Variables|/Game/OpenRPG_QuestSystem/Blueprints/Quests/BP_BaseQuest.BP_BaseQuest_C|GetCompletedGoalIndices (LocalVariables|GetLocalQuest)) (Variables|/Game/OpenRPG_QuestSystem/Blueprints/Quests/BP_BaseQuest.BP_BaseQuest_C|GetFailedGoalIndices (LocalVariables|GetLocalQuest)) (Variables|/Game/OpenRPG_QuestSystem/Blueprints/Quests/BP_BaseQuest.BP_BaseQuest_C|GetCurrentTargetAmounts (LocalVariables|GetLocalQuest)) (Variables|/Game/OpenRPG_QuestSystem/Blueprints/Quests/BP_BaseQuest.BP_BaseQuest_C|GetRemainingGoalTimes (LocalVariables|GetLocalQuest)))))
  (SaveGame|SaveGametoSlot (Variables|Save/Load|GetSaveQuestsClass) (Variables|Settings|GetSavedQuestsSlotName))
  (return))

(fn LoadQuests
  (Utilities|IsValid (Variables|Save/Load|GetSaveQuestsClass)
    (:Is%20Valid
      _)
    (:Is%20Not%20Valid
      (bind _returnvalue (SaveGame|LoadGamefromSlot (Variables|Settings|GetSavedQuestsSlotName)))
      (bind _asquest_save (Utilities|Casting|CastToQuestSave _returnvalue)
        (:then
          (Variables|Save/Load|SetSaveQuestsClass _asquest_save))
        (:CastFailed
          (return)))))
  (for _array_element (Variables|/Game/OpenRPG_QuestSystem/Blueprints/QuestSave.QuestSave_C|GetSavedQuests (Variables|Save/Load|GetSaveQuestsClass))
    (bind _output_get (LocalVariables|SetLocalSavedQuestData _array_element))
    (bind _returnvalue_2 (Game|SpawnActorfromClass (Utilities|Struct|Breaks_QuestData (Helpers|GetQuestDatafromID (Utilities|Struct|Breaks_SavedQuest _output_get))) (Math|Transform|MakeTransform "0, 0, 0" "0, 0, 0" "1,1,1") "AlwaysSpawn" 0 (Utilities|Struct|Breaks_SavedQuest _output_get) "None" (Helpers|GetQuestDatafromID (Utilities|Struct|Breaks_SavedQuest _output_get)) (Variables|Default|GetPlayer) self 0))
    (Default|LoadSavedData _returnvalue_2 (LocalVariables|GetLocalSavedQuestData))
    (Utilities|Array|Add (Variables|Quests|GetQuests) _returnvalue_2))
  (Development|PrintString "Quests Loaded Succesfully!" true true "(R=0.000000,G=0.660000,B=1.000000,A=1.000000)" 5.0)
  (return))

(fn InitializeWidgets
  (bind _foundwidgets (Widget|GetAllWidgetsOfClass (Variables|Settings|GetQuestJournalWidgetClass) false))
  (Variables|UI|SetQuestJournal (Utilities|Array|Get(acopy) _foundwidgets))
  (bind _foundwidgets_2 (Widget|GetAllWidgetsOfClass "/Game/OpenRPG_QuestSystem/UI/WB_QuestList.WB_QuestList_C" false))
  (bind _output_get (Variables|UI|SetQuestList (Utilities|Array|Get(acopy) _foundwidgets_2)))
  (Default|Initialize _output_get self (Variables|Quests|GetQuests))
  (bind _foundwidgets_3 (Class|WidgetBlueprintLibrary|GetAllWidgetswithInterface "/Game/OpenRPG_QuestSystem/Blueprints/Interfaces/BP_QuestEvents.BP_QuestEvents_C" false))
  (Variables|UI|SetQuestDetailWidgets _foundwidgets_3)
  (return))

(fn UpdateQuestWidgetDescription
  (params (Quest :type BP%20Base%20Quest%20Object%20Reference))
  (LocalVariables|SetLocalQuest Quest)
  (for _array_element (Variables|UI|GetQuestDetailWidgets)
    (Class|BPQuestEvents|OnQuestDescriptionUpdated(Message) _array_element (LocalVariables|GetLocalQuest)))
  (return))

(fn UpdateQuestGoalWidget
  (params (Quest :type BP%20Base%20Quest%20Object%20Reference) (GoalIndex :type Integer))
  (LocalVariables|SetLocalQuest Quest)
  (LocalVariables|SetLocalGoalIndex GoalIndex) ; Not used at the moment
  (for _array_element (Variables|UI|GetQuestDetailWidgets)
    (Class|BPQuestEvents|OnQuestGoalUpdated(Message) _array_element (LocalVariables|GetLocalQuest)))
  (return))

(fn UpdateSelectedQuest
  (params (Quest :type BP%20Base%20Quest%20Object%20Reference))
  (Variables|Quests|SetCurrentSelectedQuest Quest)
  (for _array_element (Variables|UI|GetQuestDetailWidgets)
    (Class|BPQuestEvents|OnQuestSelected(Message) _array_element (Variables|Quests|GetCurrentSelectedQuest)))
  (return))

(fn UpdateFinishedQuest
  (params (Quest :type BP%20Base%20Quest%20Object%20Reference))
  (LocalVariables|SetLocalQuest Quest)
  (for _array_element (Variables|UI|GetQuestDetailWidgets)
    (Class|BPQuestEvents|OnQuestFinished(Message) _array_element (LocalVariables|GetLocalQuest)))
  (return))

(fn QuestAlreadyAdded?
  (params (QuestClass :type BP%20Base%20Quest%20Class%20Reference))
  (LocalVariables|SetLocalQuest QuestClass)
  (bind _array_element (Utilities|Array|ForEachLoopwithBreak (Variables|Quests|GetQuests) :!label _label)
    (:LoopBody
      (if (== (Utilities|GetClass _array_element) (LocalVariables|GetLocalQuest))
        (LocalVariables|SetLocalAdded? true)
        (goto _label Break)))
    (:Completed
      (return (LocalVariables|GetLocalAdded?)))))

(fn UpdateQuestsList
  (Default|UpdateQuestList (Variables|UI|GetQuestList) (Variables|Quests|GetQuests))
  (return))

(fn GetFirstNPC
  (bind _output_get (LocalVariables|SetLocalNPC (Utilities|Array|Get(acopy) (Variables|NPCs|GetNearbyNPCs))))
  (Utilities|IsValid _output_get
    (:Is%20Valid
      (if (== (Utilities|Array|Length (Variables|NPCs|GetNearbyNPCs)) 1)
        (return (LocalVariables|GetLocalNPC))
        (else
          (Utilities|Array|Add (Variables|NPCs|GetNearbyNPCs) (LocalVariables|GetLocalNPC))
          (Utilities|Array|RemoveIndex (Variables|NPCs|GetNearbyNPCs))
          (return (LocalVariables|GetLocalNPC)))))
    (:Is%20Not%20Valid
      (return 0))))