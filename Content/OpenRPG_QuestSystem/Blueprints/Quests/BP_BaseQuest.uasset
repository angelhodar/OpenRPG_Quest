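; Base quest class for an RPG quest system, tracking one quest's goals, progress and description, with overridable events for child quests to script outcomes.
; EndGoal completes or fails a goal, starts followers whose prerequisites have finished, and reports updates or quest end to QuestComponent.
; A single timer tracks the shortest remaining goal time limit and fails that goal on expiry.
; State initializes from QuestData or restores from saved data.
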(event Custom|OnQuestCompleted
  ;[0.08476 0.8197 1] Overriding this events in the child quest classes, you can script everything you want for a quest to do when its completed, failed, tracked, etc.
  (CallFunction|OnGiveReward))

(event Custom|OnGoalStarted
  (params (GoalIndex :type Integer))
  ;[0.08476 0.8197 1] Overriding this events in the child quest classes, you can script everything you want for a quest to do when its completed, failed, tracked, etc.
  (Time|UpdateNewGoalTimeData GoalIndex))

(event Custom|OnQuestFailed
  ;[0.08476 0.8197 1] Overriding this events in the child quest classes, you can script everything you want for a quest to do when its completed, failed, tracked, etc.
)

(event Custom|OnGoalFailed
  (params (GoalIndex :type Integer))
  ;[0.08476 0.8197 1] Overriding this events in the child quest classes, you can script everything you want for a quest to do when its completed, failed, tracked, etc.
)

(event Custom|OnGoalCompleted
  (params (GoalIndex :type Integer))
  ;[0.08476 0.8197 1] Overriding this events in the child quest classes, you can script everything you want for a quest to do when its completed, failed, tracked, etc.
)

(event Custom|OnGiveReward
  ;[0.08476 0.8197 1] Overriding this events in the child quest classes, you can script everything you want for a quest to do when its completed, failed, tracked, etc.
)

(event Custom|OnQuestCanceled
  ;[0.08476 0.8197 1] Overriding this events in the child quest classes, you can script everything you want for a quest to do when its completed, failed, tracked, etc.
)

(fn ConstructionScript)

(fn Initialize
  (bind _questdata (Variables|Internal|GetQuestData))
  (bind (_description _startinggoalindices) (Utilities|Struct|Breaks_QuestData _questdata))
  ;[0.02946 1 0.7995] This function must be called when we spawn a quest in the world. It handles if the quest needs to load some saved data, initializes the arrays and the timer for goals with time limit
  (Variables|Default|SetCurrentDescription _description)
  (Variables|Internal|SetCurrentGoalIndices _startinggoalindices)
  (Utilities|Array|Resize (Variables|Internal|GetCurrentTargetAmounts) (Utilities|Array|Length (Utilities|Struct|Breaks_QuestData (Variables|Internal|GetQuestData))))
  (Initialization|InitializeTimer)
  (return))

(fn EndGoal
  (params (GoalIndex :type Integer) (Fail? :type Boolean))
  ;[0.313 1 0.04746] Probably the most complex function in the whole system, it will be called from the QuestManager when we have completed or failed a goal.
  (LocalVariables|SetLocalGoalIndex GoalIndex)
  (LocalVariables|SetLocalFail Fail?)
  (if (Utilities|Array|ContainsItem (Variables|Internal|GetCurrentGoalIndices) (LocalVariables|GetLocalGoalIndex)) ; First we check if the goal isnt completed or failed
    (bind _output_get (LocalVariables|SetLocalCompletedGoal (Data|GetGoalDataatIndex (LocalVariables|GetLocalGoalIndex)))) ; Extract its info
    (Managment|UpdateCurrentDescription (Utilities|Struct|Breaks_GoalData _output_get))
    (Utilities|Array|Add (select (LocalVariables|GetLocalFail) (Variables|Internal|GetFailedGoalIndices) (Variables|Internal|GetCompletedGoalIndices)) (LocalVariables|GetLocalGoalIndex)) ; We add the goal to the proper array
    (Utilities|Array|RemoveItem (Variables|Internal|GetCurrentGoalIndices) (LocalVariables|GetLocalGoalIndex)) ; Then remove it from the current goals array
    (Time|RemoveGoalTimeData (LocalVariables|GetLocalGoalIndex))
    (for _array_element (Utilities|Struct|Breaks_GoalData (LocalVariables|GetLocalCompletedGoal)) ; Now we need to iterate through the following subgoals that the ended goal starts
      (if (Managment|NeededGoalsFinished? _array_element) ; Have we finished all the goals that the following goal needs?
        (Utilities|Array|Add (Variables|Internal|GetCurrentGoalIndices) _array_element) ; If so we add it
        (CallFunction|OnGoalStarted _array_element)))
    (if (LocalVariables|GetLocalFail) ; Check which event do we have to call
      (CallFunction|OnGoalFailed (LocalVariables|GetLocalGoalIndex))
      (else
        (CallFunction|OnGoalCompleted (LocalVariables|GetLocalGoalIndex))))
    (if (or (== (LocalVariables|GetLocalGoalIndex) (Utilities|Array|LastIndex (Utilities|Struct|Breaks_QuestData (Variables|Internal|GetQuestData)))) (and (Utilities|Struct|Breaks_GoalData (LocalVariables|GetLocalCompletedGoal)) (not (LocalVariables|GetLocalFail)))) ; Now if the goal we have ended is the last goal or it completed the whole quest
      (Default|EndQuest (Variables|Default|GetQuestComponent) self "NewEnumerator1") ; Then we end this quest instance with the Completed state
      (elif (and (Utilities|Struct|Breaks_GoalData (LocalVariables|GetLocalCompletedGoal)) (LocalVariables|GetLocalFail)) ; Otherwise, if it fails the whole quest
        (Default|EndQuest (Variables|Default|GetQuestComponent) self "NewEnumerator2") ; Then we end this quest instance with the Failed state
        (else
          (Default|OnQuestGoalUpdated (Variables|Default|GetQuestComponent) self (LocalVariables|GetLocalGoalIndex))
          (return true))))
    (Utilities|Map|Clear (Variables|Internal|GetRemainingGoalTimes))
    (if (Utilities|Time|IsValidTimerHandle (Variables|Internal|GetTimeLimitChecker))
      (Utilities|Time|ClearandInvalidateTimerbyHandle (Variables|Internal|GetTimeLimitChecker))
      (return true)
      (else
        (return true)))
    (else
      (return false))))

(fn NeededGoalsFinished?
  (params (GoalIndex :type Integer))
  ;[0.1129 1 0.8601] This function checks if a goal can be started, checking if we have completed or failed all of its needed goals
  (LocalVariables|SetLocalGoalIndex GoalIndex)
  (bind _output_get (LocalVariables|SetLocalGoal (Utilities|Array|Get(acopy) (Utilities|Struct|Breaks_QuestData (Variables|Internal|GetQuestData)) (LocalVariables|GetLocalGoalIndex))))
  (bind _array_element (Utilities|Array|ForEachLoopwithBreak (Utilities|Struct|Breaks_GoalData _output_get) :!label _label)
    (:LoopBody
      (bind _output_get_2 (LocalVariables|SetLocalAllCompleted? (or (Data|IsGoalCompleted? _array_element) (Data|IsGoalFailed? _array_element))))
      (if (not _output_get_2)
        (goto _label Break)))
    (:Completed
      (return (LocalVariables|GetLocalAllCompleted?)))))

(fn IsGoalCompleted?
  (params (GoalIndex :type Integer))
  (return (Utilities|Array|ContainsItem (Variables|Internal|GetCompletedGoalIndices) GoalIndex)))

(fn GetGoalDataatIndex
  (params (Index :type Integer))
  (return (Utilities|Array|Get(acopy) (Utilities|Struct|Breaks_QuestData (Variables|Internal|GetQuestData)) Index)))

(fn IsGoalFailed?
  (params (GoalIndex :type Integer))
  (return (Utilities|Array|ContainsItem (Variables|Internal|GetFailedGoalIndices) GoalIndex)))

(fn GetGoalTargetAmount
  (params (GoalIndex :type Integer))
  (return (Utilities|Array|Get(acopy) (Variables|Internal|GetCurrentTargetAmounts) GoalIndex)))

(fn AddGoalTargetAmount
  (params (GoalIndex :type Integer) (Amount :type Integer))
  ;[0.06412 1 0.7376] This just adds an amount to the goal that we have passed
  (Utilities|Array|SetArrayElem (Variables|Internal|GetCurrentTargetAmounts) GoalIndex (+ Amount (Utilities|Array|Get(acopy) (Variables|Internal|GetCurrentTargetAmounts) GoalIndex)))
  (return))

(fn HandleGoalTimes
  (Managment|EndGoal (Variables|Internal|GetNextShortestGoalTimeIndex) true)
  (return))

(fn GetGoalRemainingTime
  (params (GoalIndex :type Integer))
  (return (- (.Value (Utilities|Map|Find (Variables|Internal|GetRemainingGoalTimes) GoalIndex)) (Class|KismetSystemLibrary|GetTimerElapsedTimeHandle (Variables|Internal|GetTimeLimitChecker)))))

(fn LoadSavedData
  (params (Data :type S%20Saved%20Quest%20Structure))
  ;[0.03439 1 0.2406] This will fill the variables with the saved data
  (bind _output_get (LocalVariables|SetLocalData Data))
  (Variables|Default|SetID (.ID (Utilities|Struct|Breaks_SavedQuest _output_get)))
  (Variables|Internal|SetState (.State (Utilities|Struct|Breaks_SavedQuest _output_get)))
  (Variables|Default|SetCurrentDescription (.CurrentDescription (Utilities|Struct|Breaks_SavedQuest _output_get)))
  (Variables|Internal|SetCurrentGoalIndices (.CurrentGoalIndices (Utilities|Struct|Breaks_SavedQuest (LocalVariables|GetLocalData))))
  (Variables|Internal|SetCompletedGoalIndices (.CompletedGoalIndices (Utilities|Struct|Breaks_SavedQuest (LocalVariables|GetLocalData))))
  (Variables|Internal|SetFailedGoalIndices (.FailedGoalIndices (Utilities|Struct|Breaks_SavedQuest (LocalVariables|GetLocalData))))
  (Variables|Internal|SetCurrentTargetAmounts (.CurrentTargetAmounts (Utilities|Struct|Breaks_SavedQuest (LocalVariables|GetLocalData))))
  (Variables|Internal|SetRemainingGoalTimes (.RemainingGoalTimes (Utilities|Struct|Breaks_SavedQuest (LocalVariables|GetLocalData))))
  (Initialization|InitializeTimer)
  (return))

(fn UpdateNewGoalTimeData
  (params (Index :type Integer))
  (bind _output_get (LocalVariables|SetLocalGoalIndex Index))
  (if (!= (Utilities|Struct|Breaks_GoalData (Data|GetGoalDataatIndex _output_get)) -1)
    (Time|UpdateGoalsRemainingTime)
    (Utilities|Map|Add (Variables|Internal|GetRemainingGoalTimes) (LocalVariables|GetLocalGoalIndex) (Math|Conversions|ToFloat(Integer) (Utilities|Struct|Breaks_GoalData (Data|GetGoalDataatIndex _output_get))))
    (Time|UpdateShortestRemainingGoalTime)
    (return)
    (else
      (return))))

(fn InitializeTimer
  (bind _returnvalue (Utilities|Time|SetTimerbyFunctionName 0 "UpdateTimeLimits" 1.0 true))
  (bind _output_get (Variables|Internal|SetTimeLimitChecker _returnvalue))
  (Utilities|Time|PauseTimerbyHandle _output_get)
  (for _array_element (Variables|Internal|GetCurrentGoalIndices)
    (CallFunction|OnGoalStarted _array_element))
  (return))

(fn UpdateShortestRemainingGoalTime
  (bind _keys (Utilities|Map|Keys (Variables|Internal|GetRemainingGoalTimes)))
  (for _array_element _keys
    (bind _output_get (LocalVariables|SetLocalCurrentGoalIndex _array_element))
    (bind _output_get_2 (LocalVariables|SetLocalGoalRemainingTime (.Value (Utilities|Map|Find (Variables|Internal|GetRemainingGoalTimes) _output_get))))
    (if (< _output_get_2 (LocalVariables|GetLocalMinimumRemainingTime))
      (LocalVariables|SetLocalMinimumRemainingTime (LocalVariables|GetLocalGoalRemainingTime))
      (Variables|Internal|SetNextShortestGoalTimeIndex (LocalVariables|GetLocalCurrentGoalIndex))))
  (bind _returnvalue (Utilities|Time|SetTimerbyFunctionName 0 "HandleGoalTimes" (LocalVariables|GetLocalMinimumRemainingTime)))
  (Variables|Internal|SetTimeLimitChecker _returnvalue)
  (return))

(fn UpdateGoalsRemainingTime
  (bind _keys (Utilities|Map|Keys (Variables|Internal|GetRemainingGoalTimes)))
  (for _array_element _keys
    (bind _output_get (LocalVariables|SetLocalCurrentGoalIndex _array_element))
    (bind _output_get_2 (LocalVariables|SetLocalGoalRemainingTime (.Value (Utilities|Map|Find (Variables|Internal|GetRemainingGoalTimes) _output_get))))
    (Utilities|Map|Add (Variables|Internal|GetRemainingGoalTimes) (LocalVariables|GetLocalCurrentGoalIndex) (Math|Float|Clamp(Float) (- _output_get_2 (Class|KismetSystemLibrary|GetTimerElapsedTimeHandle (Variables|Internal|GetTimeLimitChecker))) (Utilities|Time|GetWorldDeltaSeconds) (- _output_get_2 (Class|KismetSystemLibrary|GetTimerElapsedTimeHandle (Variables|Internal|GetTimeLimitChecker))))))
  (return))

(fn RemoveGoalTimeData
  (params (GoalIndex :type Integer))
  (bind _output_get (LocalVariables|SetLocalGoalIndex GoalIndex))
  (Utilities|Map|Remove (Variables|Internal|GetRemainingGoalTimes) _output_get)
  (if (!= (Utilities|Map|Length (Variables|Internal|GetRemainingGoalTimes)) 0)
    (Time|UpdateGoalsRemainingTime)
    (Time|UpdateShortestRemainingGoalTime)
    (return)
    (else
      (Utilities|Time|ClearandInvalidateTimerbyHandle (Variables|Internal|GetTimeLimitChecker))
      (return))))

(fn UpdateCurrentDescription
  (params (NewText :type Text))
  (bind _output_get (LocalVariables|SetLocalText NewText))
  (if (Utilities|Text|TextIsEmpty _output_get) ; Does the goal updates the description of the quest in the quest menu?
    _
    (else
      (Variables|Default|SetCurrentDescription (Utilities|Text|FormatText "{Current}{Updated}" (Variables|Default|GetCurrentDescription) (LocalVariables|GetLocalText))) ; Now we have updated the current description
      (Default|OnQuestDescriptionUpdated (Variables|Default|GetQuestComponent) self)))
  (return))