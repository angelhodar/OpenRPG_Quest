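; Actor component that makes its owner a quest interactable, working out which quest indicator it should present.
; On BeginPlay it loads indicator priority, quests to accept or finish, and goals to progress from a DataTable row.
; It queries the passed-in quest manager in priority order and takes the first matching state with its ID.
; UpdateQuestIndicatorState broadcasts that state and quest ID through an indicator-changed dispatcher.
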(event Custom|RefreshQuestIndicatorState
  (params (NewState :type e_QuestIndicatorState%20Enum :default "NewEnumerator0") (QuestID :type Name))
  (Default|CallOnQuestIndicatorStateChanged NewState QuestID))

(event EventBeginPlay
  (bind _datatable (Variables|Default|GetDataTable))
  (Utilities|IsValid _datatable
    (:Is%20Valid
      (bind _returnvalue (Utilities|GetDataTableRow _datatable (Variables|Default|GetTableRow))
        (:then
          (Variables|Default|SetQuestIndicatorPriority (.IndicatorPriority (Utilities|Struct|Breaks_QuestInteractable _returnvalue)))
          (Variables|Default|SetQuestsToAccept (.QuestsToAccept (Utilities|Struct|Breaks_QuestInteractable _returnvalue)))
          (Variables|Default|SetQuestsToFinish (.QuestsToFinish (Utilities|Struct|Breaks_QuestInteractable _returnvalue)))
          (Variables|Default|SetGoalsToProgress (.GoalsToComplete (Utilities|Struct|Breaks_QuestInteractable _returnvalue))))
        (:RowNotFound
          (Development|PrintString (Utilities|String|Append "Row not valid in quest interactable of " (Utilities|GetDisplayName (Components|GetOwner))) true true "(R=1.000000,G=0.000000,B=0.024480,A=1.000000)"))))
    (:Is%20Not%20Valid
      (Development|PrintString (Utilities|String|Append "Datatable not valid in quest interactable component of " (Utilities|GetDisplayName (Components|GetOwner))) true true "(R=1.000000,G=0.000000,B=0.024480,A=1.000000)"))))

(fn CanFinishQuest?
  (params (QuestManager :type BPC%20Player%20Quest%20Manager%20Object%20Reference))
  (LocalVariables|SetLocalQuestManager QuestManager)
  (bind _array_element (Utilities|Array|ForEachLoopwithBreak (Variables|Default|GetQuestsToFinish) :!label _label)
    (:LoopBody
      (bind _output_get (LocalVariables|SetLocalQuest _array_element))
      (bind _output_get_2 (LocalVariables|SetLocalHasFinisableQuest? (Utilities|Enum|Equal(Enum) (Default|GetQuestState (LocalVariables|GetLocalQuestManager) _output_get) "NewEnumerator4")))
      (if _output_get_2
        (goto _label Break)))
    (:Completed
      (return (LocalVariables|GetLocalHasFinisableQuest?) (LocalVariables|GetLocalQuest)))))

(fn CanAcceptQuest?
  (params (QuestMananger :type BPC%20Player%20Quest%20Manager%20Object%20Reference))
  (LocalVariables|SetLocalQuestManager QuestMananger)
  (bind _array_element (Utilities|Array|ForEachLoopwithBreak (Variables|Default|GetQuestsToAccept) :!label _label)
    (:LoopBody
      (bind _output_get (LocalVariables|SetLocalQuest _array_element))
      (bind _output_get_2 (LocalVariables|SetLocalHasQuestToAccept? (Default|QuestCanbeAccepted? (LocalVariables|GetLocalQuestManager) _output_get)))
      (if _output_get_2
        (goto _label Break)))
    (:Completed
      (return (LocalVariables|GetLocalHasQuestToAccept?) (LocalVariables|GetLocalQuest)))))

(fn CanProgressGoal?
  (params (QuestManager :type BPC%20Player%20Quest%20Manager%20Object%20Reference))
  (LocalVariables|SetLocalQuestManager QuestManager)
  (bind _array_element (Utilities|Array|ForEachLoopwithBreak (Variables|Default|GetGoalsToProgress) :!label _label)
    (:LoopBody
      (bind _output_get (LocalVariables|SetLocalGoal _array_element))
      (bind _output_get_2 (LocalVariables|SetHasGoalToProgress? (Default|IsGoalActive? (LocalVariables|GetLocalQuestManager) _output_get)))
      (if _output_get_2
        (goto _label Break)))
    (:Completed
      (return (LocalVariables|GetHasGoalToProgress?) (LocalVariables|GetLocalGoal)))))

(fn GetHighestPriorityQuestIndicatorState
  (params (QuestManager :type BPC%20Player%20Quest%20Manager%20Object%20Reference))
  (LocalVariables|SetLocalQuestManager QuestManager)
  (bind _array_element (Utilities|Array|ForEachLoopwithBreak (Variables|Default|GetQuestIndicatorPriority) :!label _label)
    (:LoopBody
      (switch Utilities|FlowControl|Switch|Switchone_QuestIndicatorState _array_element
        (:NewEnumerator0
          (if (.Out (CallFunction|CanFinishQuest? (LocalVariables|GetLocalQuestManager)))
            (LocalVariables|SetLocalQuestIndicator "NewEnumerator0")
            (LocalVariables|SetLocalID (.QuestID (CallFunction|CanFinishQuest? (LocalVariables|GetLocalQuestManager))))
            (goto _label Break)))
        (:NewEnumerator1
          (if (.Out (CallFunction|CanProgressGoal? (LocalVariables|GetLocalQuestManager)))
            (LocalVariables|SetLocalQuestIndicator "NewEnumerator1")
            (LocalVariables|SetLocalID (.Goal (CallFunction|CanProgressGoal? (LocalVariables|GetLocalQuestManager))))
            (goto _label Break)))
        (:NewEnumerator2
          (if (.Out (CallFunction|CanAcceptQuest? (LocalVariables|GetLocalQuestManager)))
            (LocalVariables|SetLocalQuestIndicator "NewEnumerator2")
            (LocalVariables|SetLocalID (.QuestID (CallFunction|CanAcceptQuest? (LocalVariables|GetLocalQuestManager))))
            (goto _label Break)))
        (:NewEnumerator3
          (LocalVariables|SetLocalQuestIndicator "NewEnumerator3"))))
    (:Completed
      (if (Utilities|Enum|Equal(Enum) (LocalVariables|GetLocalQuestIndicator) "NewEnumerator1")
        (return (LocalVariables|GetLocalQuestIndicator) (Default|GetQuestwithActiveGoal (LocalVariables|GetLocalQuestManager) (LocalVariables|GetLocalID)) (LocalVariables|GetLocalID))
        (else
          (return (LocalVariables|GetLocalQuestIndicator) (LocalVariables|GetLocalID) "None"))))))

(fn UpdateQuestIndicatorState
  (params (QuestManager :type BPC%20Player%20Quest%20Manager%20Object%20Reference))
  (bind _output_get (LocalVariables|SetLocalQuestManager QuestManager))
  (CallFunction|RefreshQuestIndicatorState (.IndicatorState (CallFunction|GetHighestPriorityQuestIndicatorState _output_get)) (.QuestID (CallFunction|GetHighestPriorityQuestIndicatorState _output_get)))
  (return))