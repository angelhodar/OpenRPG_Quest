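; BPL_Quest is a Blueprint function library of shared helpers for the OpenRPG quest system.
; It fetches the quest manager component from player character 0 and looks up static quest definitions by ID in the DT_Quests data table.
; Goal required amounts are read through that same row lookup.
; Two Select-based helpers map quest category and quest state to fixed colors.
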(fn GetPlayerQuestManagerComponent
  (return (Actor|GetComponentbyClass (Game|GetPlayerCharacter (LocalVariables|Get__WorldContext)) "/Game/OpenRPG_Quests/Blueprints/BPC_PlayerQuestManager.BPC_PlayerQuestManager_C")))

(fn GetStaticQuestDatabyID
  (params (QuestID :type Name))
  (bind _returnvalue (Utilities|GetDataTableRow "/Game/OpenRPG_Quests/Datatables/DT_Quests.DT_Quests" QuestID)
    (:then
      (return _returnvalue))
    (:RowNotFound
      (return ""))))

(fn GetQuestGoalRequiredAmount
  (params (QuestID :type Name) (GoalID :type Name))
  (return (Utilities|Struct|Breaks_QuestGoal (.Value (Utilities|Map|Find (Utilities|Struct|Breaks_StaticQuestData (CallFunction|GetStaticQuestDatabyID QuestID)) GoalID)))))

(fn GetColorbyQuestCategory
  (params (Category :type e_QuestCategory%20Enum :default "NewEnumerator0"))
  (return (Utilities|Select :Index Category :NewEnumerator0 "(R=0.953125,G=0.939271,B=0.000000,A=1.000000)" :NewEnumerator1 "(R=0.000000,G=0.430671,B=1.000000,A=1.000000)" :NewEnumerator2 "(R=0.160640,G=1.000000,B=0.000000,A=1.000000)")))

(fn GetColorbyQuestState
  (params (State :type e_QuestState%20Enum :default "NewEnumerator6"))
  (return (Utilities|Select :Index State :NewEnumerator6 "(R=0.281250,G=0.281250,B=0.281250,A=1.000000)" :NewEnumerator0 "(R=1.000000,G=1.000000,B=1.000000,A=1.000000)" :NewEnumerator2 "(R=0.937500,G=0.000000,B=0.000000,A=1.000000)" :NewEnumerator4 "(R=0.019947,G=0.960200,B=1.000000,A=1.000000)" :NewEnumerator5 "(R=0.000000,G=1.000000,B=0.119515,A=1.000000)")))